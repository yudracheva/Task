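; Player controller that toggles a free-flight state and moves the view between BP_House actors in the level.
; BeginPlay gathers all houses, and GetNextHouse steps through that array, wrapping to the first and starting there when no current house is valid.
; Switching to a house stops free flight, calls MakeUnselected on it, blends the view target to it and stores its camera's world transform.
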(event `self.ReceiveBeginPlay`
  (bind _outactors (`GameplayStatics.GetAllActorsOfClass` "/Game/Blueprints/BP_House.BP_House_C"))
  (set `self.House` _outactors))

(event `StopFreeFlight`
  (set `self.isFreeFlightEnabled` false))

(event `StartFreeFlight`
  (set `self.isFreeFlightEnabled` true))

(fn `GetFreeFlightState`
  (returns (Enabled :type Boolean))
  (return (`self.isFreeFlightEnabled`)))

(fn `GetNextHouse`
  (returns (House :type "/Game/Blueprints/BP_House Object Reference"))
  (bind _house (`self.House`))
  (bind _house_2 (`self.House`))
  (`/Engine/EditorBlueprintResources/StandardMacros.IsValid` (`self.CurrentHouse`)
    (:`Is Valid`
      (bind _result (`/Engine/EditorBlueprintResources/StandardMacros.IncrementInt` (`KismetArrayLibrary.Array_Find` _house_2 (`self.CurrentHouse`)))
        (:`  `
          (if (== (`KismetArrayLibrary.Array_Length` _house_2) _result)
            (return (`|GetArrayItem` _house))
            (else
              (return (`|GetArrayItem` _house _result)))))))
    (:`Is Not Valid`
      (return (`|GetArrayItem` (`self.House`))))))

(fn `SwitchCameraToHouseCamera`
  (params (House :type "/Game/Blueprints/BP_House Object Reference"))
  (`self.StopFreeFlight`)
  (`/Game/Blueprints/BP_House.MakeUnselected` House)
  (bind _output_get (set `self.CurrentHouse` House))
  (`self.SetViewTargetWithBlend` _output_get 2.0)
  (set `self.HouseTransform` (`SceneComponent.K2_GetComponentToWorld` (`/Game/Blueprints/BP_House.Camera` _output_get))))

(fn `UserConstructionScript`)