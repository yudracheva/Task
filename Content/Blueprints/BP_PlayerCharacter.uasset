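; Player character that moves and looks around via axis inputs, including vertical movement, and lets the player pick houses by looking at them.
; While the player controller reports free-flight state, Tick line-traces forward from the main camera, toggles selection on the traced BP_House and fires could/could-not-be-selected calls when the target changes.
; Pressing Q asks the player controller to switch to the traced house's camera.
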(event `self.ReceiveBeginPlay`
  (bind _asbp_player_controller (cast `/Game/Blueprints/BP_PlayerController` (`GameplayStatics.GetPlayerController` 0)))
  (set `self.Player Controller` _asbp_player_controller))

(event `InputAxis|MoveForward`
  (params (AxisValue :type "Float (single-precision)"))
  (`self.AddMovementInput` (`SceneComponent.GetForwardVector` (`self.MainCamera`)) AxisValue))

(event `InputAxis|MoveRight`
  (params (AxisValue :type "Float (single-precision)"))
  (`self.AddMovementInput` (`self.GetActorRightVector`) AxisValue))

(event `InputAxis|MoveUP`
  (params (AxisValue :type "Float (single-precision)"))
  (`self.AddMovementInput` (`self.GetActorUpVector`) AxisValue))

(event `InputAxis|LookUp`
  (params (AxisValue :type "Float (single-precision)"))
  (`self.AddControllerPitchInput` AxisValue))

(event `InputAxis|LookRight`
  (params (AxisValue :type "Float (single-precision)"))
  (`self.AddControllerYawInput` AxisValue))

(event `self.ReceiveTick`
  (params (DeltaSeconds :type "Float (single-precision)"))
  (bind _maincamera (`self.MainCamera`))
  (bind _tracedhouse (`self.TracedHouse`))
  (bind _returnvalue (`SceneComponent.K2_GetComponentLocation` _maincamera))
  (if (`/Game/Blueprints/BP_PlayerController.GetFreeFlightState` (`self.Player Controller`))
    (bind _outhit (`KismetSystemLibrary.LineTraceSingle` :`Start` _returnvalue :`End` (+ _returnvalue (* (`KismetMathLibrary.GetForwardVector` (`SceneComponent.K2_GetComponentRotation` _maincamera)) 1500.0)) :`TraceChannel` "TraceTypeQuery1" :`DrawDebugType` "ForOneFrame"))
    (bind (_bblockinghit _binitialoverlap _time _distance _location _impactpoint _normal _impactnormal _physmat _hitactor) (`GameplayStatics.BreakHitResult` _outhit))
    (if (not (== _tracedhouse _hitactor))
      (`/Engine/EditorBlueprintResources/StandardMacros.IsValid` _tracedhouse
        (:`Is Valid`
          (`/Game/Blueprints/BP_House.MakeUnselected` _tracedhouse))
        (:`Is Not Valid`
          _))
      (bind _asbp_house (cast `/Game/Blueprints/BP_House` _hitactor)
        (:`then`
          (bind _output_get (set `self.TracedHouse` _asbp_house))
          (`/Game/Blueprints/BP_House.MakeSelected` _output_get)
          (`self.HouseCouldBeSelected`))
        (:`CastFailed`
          (set `self.TracedHouse` null)
          (`self.HouseCouldNotBeSelected`))))))

(event `Key|Q`
  (params (Key :type "Key Structure"))
  (bind _tracedhouse (`self.TracedHouse`))
  (:`Pressed`
    (`/Engine/EditorBlueprintResources/StandardMacros.IsValid` _tracedhouse
      (:`Is Valid`
        (`/Game/Blueprints/BP_PlayerController.SwitchCameraToHouseCamera` (`self.Player Controller`) _tracedhouse)))))

(fn `UserConstructionScript`)