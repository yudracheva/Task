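; Traffic light actor that cycles its lamps and stops or releases BP_Car actors entering its trigger box.
; A looping Delay and FlipFlop sequence on BeginPlay alternates green and red with yellow between, holding red longest, and toggles lamp visibility.
; Yellow and green both set the boolean go state.
; On overlap, a car drives on go, otherwise it stops and a Retriggerable Delay loop rechecks until the state changes.
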(event `self.ReceiveBeginPlay`
  (`KismetSystemLibrary.Delay` 2.0 :!label _label)
  (`self.SwitchToYellow`)
  (`KismetSystemLibrary.Delay` 2.0)
  (`/Engine/EditorBlueprintResources/StandardMacros.FlipFlop`
    (:`A`
      (`self.SwitchToGreen`)
      (goto _label))
    (:`B`
      (`self.SwitchToRed`)
      (`KismetSystemLibrary.Delay` 10.0)
      (goto _label))))

(event `self.Box.OnComponentBeginOverlap`
  (params (OverlappedComponent :type "PrimitiveComponent Object Reference") (OtherActor :type "Actor Object Reference") (OtherComp :type "PrimitiveComponent Object Reference") (OtherBodyIndex :type Integer) (bFromSweep :type Boolean) (SweepResult :type "HitResult Structure (by ref)"))
  (bind _asbp_car (cast `/Game/Blueprints/BP_Car` OtherActor))
  (if (`self.TrafficLightsState`) :!label _label_2
    (`/Game/Blueprints/BP_Car.Driving` _asbp_car)
    (else
      (`/Game/Blueprints/BP_Car.Stop` _asbp_car)
      (`KismetSystemLibrary.RetriggerableDelay` 0.2)
      (goto _label_2))))

(fn `SwitchToGreen`
  (set `self.TrafficLightsState` true)
  (`|ExecutionSequence`
    (:`then_0`
      (`SceneComponent.SetHiddenInGame` (`self.GreenLight`) false false)
      (`SceneComponent.SetHiddenInGame` (`self.GreenLight1`) false false)
      (`SceneComponent.SetHiddenInGame` (`self.GreenLight2`) false false))
    (:`then_1`
      (`SceneComponent.SetHiddenInGame` (`self.RedLight`) true false)
      (`SceneComponent.SetHiddenInGame` (`self.RedLight1`) true false)
      (`SceneComponent.SetHiddenInGame` (`self.RedLight2`) true false)
      (`SceneComponent.SetHiddenInGame` (`self.YellowLight`) true false)
      (`SceneComponent.SetHiddenInGame` (`self.YellowLight1`) true false)
      (`SceneComponent.SetHiddenInGame` (`self.YellowLight2`) true false))))

(fn `SwitchToRed`
  (set `self.TrafficLightsState` false)
  (`|ExecutionSequence`
    (:`then_0`
      (`SceneComponent.SetHiddenInGame` (`self.RedLight`) false false)
      (`SceneComponent.SetHiddenInGame` (`self.RedLight1`) false false)
      (`SceneComponent.SetHiddenInGame` (`self.RedLight2`) false false))
    (:`then_1`
      (`SceneComponent.SetHiddenInGame` (`self.YellowLight`) true false)
      (`SceneComponent.SetHiddenInGame` (`self.YellowLight1`) true false)
      (`SceneComponent.SetHiddenInGame` (`self.YellowLight2`) true false)
      (`SceneComponent.SetHiddenInGame` (`self.GreenLight`) true false)
      (`SceneComponent.SetHiddenInGame` (`self.GreenLight1`) true false)
      (`SceneComponent.SetHiddenInGame` (`self.GreenLight2`) true false))))

(fn `SwitchToYellow`
  (set `self.TrafficLightsState` true)
  (`|ExecutionSequence`
    (:`then_0`
      (`SceneComponent.SetHiddenInGame` (`self.YellowLight`) false false)
      (`SceneComponent.SetHiddenInGame` (`self.YellowLight1`) false false)
      (`SceneComponent.SetHiddenInGame` (`self.YellowLight2`) false false))
    (:`then_1`
      (`SceneComponent.SetHiddenInGame` (`self.GreenLight`) true false)
      (`SceneComponent.SetHiddenInGame` (`self.GreenLight1`) true false)
      (`SceneComponent.SetHiddenInGame` (`self.GreenLight2`) true false)
      (`SceneComponent.SetHiddenInGame` (`self.RedLight`) true false)
      (`SceneComponent.SetHiddenInGame` (`self.RedLight1`) true false)
      (`SceneComponent.SetHiddenInGame` (`self.RedLight2`) true false))))

(fn `UserConstructionScript`)