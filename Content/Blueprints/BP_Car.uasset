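; BP_Car is a traffic car that drives along a spline and picks a random mesh from an array on BeginPlay.
; MoveSpline takes a spline, start point and speed, then advances distance each frame through a looping zero-length Delay instead of Tick.
; At the spline's end it teleports back to the start.
; Any Box overlap sets Stand, pausing movement with 0.2-second polling until an end overlap clears it.
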(event `self.ReceiveBeginPlay`
  (`self.SetMesh`))

(event `MoveSpline`
  (params (Spline :type "/Game/Blueprints/BP_TrafficSpline Object Reference") (StartPoint :type Integer) (Speed :type "Float (double-precision)"))
  (bind _spline (`/Game/Blueprints/BP_TrafficSpline.Spline` Spline))
  (bind _distancealongspline (`self.DistanceAlongSpline`))
  (bind (_returnvalue_location _returnvalue_rotation) (`KismetMathLibrary.BreakTransform` (`SplineComponent.GetTransformAtDistanceAlongSpline` _spline (`self.DistanceAlongSpline`) "World" false)))
  (bind (_returnvalue_location_2 _returnvalue_rotation_2) (`KismetMathLibrary.BreakTransform` (`SplineComponent.GetTransformAtDistanceAlongSpline` _spline (`self.DistanceAlongSpline`) "World" false)))
  (set `self.CurrentSpeed` Speed)
  (set `self.DistanceAlongSpline` (`SplineComponent.GetDistanceAlongSplineAtSplinePoint` _spline StartPoint))
  (`self.K2_SetActorTransform` (`KismetMathLibrary.MakeTransform` _returnvalue_location_2 _returnvalue_rotation_2) false true :!label _label)
  (`self.K2_SetActorLocationAndRotation` _returnvalue_location _returnvalue_rotation :!label _label_2)
  (if (`self.Stand`) :!label _label_3
    (`KismetSystemLibrary.Delay` 0.2)
    (goto _label_3)
    (else
      (set `self.DistanceAlongSpline` (+ _distancealongspline (* (`self.CurrentSpeed`) (`GameplayStatics.GetWorldDeltaSeconds`))))
      (if (<= (- (`SplineComponent.GetSplineLength` _spline) _distancealongspline) 0.0)
        (set `self.DistanceAlongSpline` 0.0)
        (goto _label)
        (else
          (`KismetSystemLibrary.Delay` 0.0)
          (goto _label_2))))))

(event `self.Box.OnComponentBeginOverlap`
  (params (OverlappedComponent :type "PrimitiveComponent Object Reference") (OtherActor :type "Actor Object Reference") (OtherComp :type "PrimitiveComponent Object Reference") (OtherBodyIndex :type Integer) (bFromSweep :type Boolean) (SweepResult :type "HitResult Structure (by ref)"))
  (`self.Stop`))

(event `self.Box.OnComponentEndOverlap`
  (params (OverlappedComponent :type "PrimitiveComponent Object Reference") (OtherActor :type "Actor Object Reference") (OtherComp :type "PrimitiveComponent Object Reference") (OtherBodyIndex :type Integer))
  (`self.Driving`))

(fn `Driving`
  (set `self.Stand` false))

(fn `GetRandomMesh`
  (returns (RandomMaterial :type "StaticMesh Object Reference"))
  (bind _staticmesharray (`self.StaticMeshArray`))
  (bind _returnvalue (`KismetArrayLibrary.Array_Length` _staticmesharray))
  (if (> _returnvalue 0)
    (return (`|GetArrayItem` _staticmesharray (`KismetMathLibrary.RandomIntegerInRange` 0 (- _returnvalue 1))))
    (else
      (return null))))

(fn `SetMesh`
  (bind _randommaterial (`self.GetRandomMesh`))
  (if (!= _randommaterial null)
    (`StaticMeshComponent.SetStaticMesh` (`self.StaticMesh`) _randommaterial)
    (return)
    (else
      (return))))

(fn `Stop`
  (set `self.Stand` true))

(fn `UserConstructionScript`
  (`parent.UserConstructionScript`))