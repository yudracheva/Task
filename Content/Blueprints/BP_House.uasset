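; BP_House is a selectable house with an orbit camera and an adjustable material.
; Look axes rotate the camera boom, and the mouse wheel changes its clamped arm length for zoom.
; BeginPlay creates a dynamic material instance, which selection functions swap with a highlight material.
; Parameter functions write the blue channel of "Param" on that instance, but read from a parameter named "None".
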(event `self.ReceiveBeginPlay`
  (bind _asmaterial_instance (cast `MaterialInstance` (`|GetArrayItem` (`MeshComponent.GetMaterials` (`self.StaticMesh`)))))
  (bind _output_get (set `self.DefaultMaterial` _asmaterial_instance))
  (bind _returnvalue (`PrimitiveComponent.CreateDynamicMaterialInstance` (`self.StaticMesh`) 0 _output_get "None"))
  (set `self.DefaultMaterialInstance` _returnvalue))

(event `InputAxisKey|MouseWheelAxis`
  (params (AxisValue :type "Float (single-precision)"))
  (`self.ChangeZoomValue` AxisValue))

(event `InputAxis|LookUp`
  (params (AxisValue :type "Float (single-precision)"))
  (bind _returnvalue (`SceneComponent.GetRelativeTransform` (`self.CameraBoom`)))
  (`SceneComponent.K2_SetRelativeRotation` (`self.CameraBoom`) (`KismetMathLibrary.MakeRotator` (.roll (.rotation _returnvalue)) (+ (* 2 AxisValue) (.pitch (.rotation _returnvalue))) (.yaw (.rotation _returnvalue))) false false))

(event `InputAxis|LookRight`
  (params (AxisValue :type "Float (single-precision)"))
  (bind _returnvalue (`SceneComponent.GetRelativeTransform` (`self.CameraBoom`)))
  (`SceneComponent.K2_SetRelativeRotation` (`self.CameraBoom`) (`KismetMathLibrary.MakeRotator` (.roll (.rotation _returnvalue)) (.pitch (.rotation _returnvalue)) (+ (.yaw (.rotation _returnvalue)) (* 2 AxisValue))) false false))

(fn `ChangeMaterialParameter`
  (params (Input :type "Float (double-precision)"))
  (bind _returnvalue (`MaterialInstanceDynamic.K2_GetVectorParameterValue` (`self.DefaultMaterialInstance`) "None"))
  (`MaterialInstanceDynamic.SetVectorParameterValue` (`self.DefaultMaterialInstance`) "Param" (make `LinearColor` (break `LinearColor` _returnvalue) (`.G` (break `LinearColor` _returnvalue)) Input (`.A` (break `LinearColor` _returnvalue)))))

(fn `ChangeZoomValue`
  (params (AxisValue :type "Float (double-precision)"))
  (set `SpringArmComponent.TargetArmLength` (`KismetMathLibrary.FClamp` (+ (* AxisValue -10.0) (`SpringArmComponent.TargetArmLength` (`self.CameraBoom`))) 100.0 500.0) (`self.CameraBoom`)))

(fn `GetCurrentMaterialParameter`
  (returns (Parameter :type "Float (double-precision)"))
  (bind _returnvalue (`MaterialInstanceDynamic.K2_GetVectorParameterValue` (`self.DefaultMaterialInstance`) "None"))
  (return (`.B` (break `LinearColor` _returnvalue))))

(fn `MakeSelected`
  (`PrimitiveComponent.SetMaterial` (`self.StaticMesh`) 0 (`self.SelectedMaterial`)))

(fn `MakeUnselected`
  (`PrimitiveComponent.SetMaterial` (`self.StaticMesh`) 0 (`self.DefaultMaterialInstance`)))

(fn `UserConstructionScript`)